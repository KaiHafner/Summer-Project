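; BP_LobbyPC is the lobby player controller that sets up each local player's lobby screen and registers them with the game mode.
; On BeginPlay, the local controller shows the cursor, adds WB_LobbyUI to the viewport and calls SetPlayerNameOnServer with text from the game instance.
; That event asks BP_LobbyGM to update this player's lobby info, without using the passed name.
; RetryUpdateLobbyInfo repeats the update after a short delay.
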(event `self.ReceiveBeginPlay`
  (`self.SetUp`))

(event `SetPlayerNameOnServer`
  (params (PlayerName :type Text))
  (bind _asbp_lobby_gm (cast `/Game/Blueprints/Lobby/BP_LobbyGM` (`GameplayStatics.GetGameMode`)))
  (`/Game/Blueprints/Lobby/BP_LobbyGM.UpdatePlayerLobbyInfo` _asbp_lobby_gm self))

(event `RetryUpdateLobbyInfo`
  (`KismetSystemLibrary.Delay` 0.1)
  (bind _asbp_lobby_gm (cast `/Game/Blueprints/Lobby/BP_LobbyGM` (`GameplayStatics.GetGameMode`)))
  (`/Game/Blueprints/Lobby/BP_LobbyGM.UpdatePlayerLobbyInfo` _asbp_lobby_gm self))

(fn `SetUp`
  (if (`self.IsLocalPlayerController`)
    (set `self.bShowMouseCursor` true)
    (`WidgetBlueprintLibrary.SetInputMode_GameAndUIEx` self (`self.Lobby UI`) "DoNotLock" false)
    (bind _returnvalue (`|CreateWidget` "/Game/Blueprints/Lobby/UI/WB_LobbyUI.WB_LobbyUI_C"))
    (bind _output_get (set `self.Lobby UI` _returnvalue))
    (`UserWidget.AddToViewport` _output_get 0)
    (`self.SetPlayerNameOnServer` (`KismetTextLibrary.Conv_ObjectToText` (cast `/Game/Blueprints/BP_GameInstance` (`GameplayStatics.GetGameInstance`) :!pure true)))))

(fn `UserConstructionScript`)